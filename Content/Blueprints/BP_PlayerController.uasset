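; Player controller that boots the game into a mouse-driven UI built on the BP_LC_Main widget.
; BeginPlay creates and stores that widget, adds it to the viewport, sets UI-only input focused on it and shows the cursor.
; An Escape key binding quits the game.
; A separate LoadBytesFromFile helper reads a file by directory and name and returns its bytes on success; nothing in this graph calls it.
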(event EventBeginPlay
  (bind _returnvalue (UserInterface|CreateWidget "/Game/UI/BP_LC_Main.BP_LC_Main_C" self))
  (bind _output_get (Variables|Default|SetMainWidget _returnvalue))
  (UserInterface|Viewport|AddtoViewport _output_get 0)
  (Input|SetInputModeUIOnly self (Variables|Default|GetMainWidget) "DoNotLock")
  (Variables|Default|SetbShowMouseCursor true))

(event Input|KeyboardEvents|Escape
  (params (Key :type Key%20Structure :default "None"))
  (:Pressed
    (Game|QuitGame self "Quit" false)))

(fn ConstructionScript)

(fn LoadBytesfromFile
  (params (DirPath :type String) (FileName :type String))
  (bind (_bsuccess _readfile) (Class|EFMBPLibrary|ReadFile DirPath FileName))
  (if _bsuccess
    (return (Class|EFMFile|GetBytes _readfile))))