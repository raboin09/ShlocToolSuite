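; BP_Utils is a utility Blueprint that resolves on-disk paths for the game's data and font folders.
; GetDataPath maps a folder type to its subfolder and appends it to the game or uproject root, depending on whether the build is packaged.
; GetFullFilePathList uses it to list every file in the element data folder as full paths.
; A helper fetches player 0's BP_PlayerController, and the CSV-load callbacks are empty stubs.
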(fn GetDataPath
  (params (FolderName :type DataFolderEnum%20Enum :default "NewEnumerator0"))
  (bind _outcontroller (CallFunction|GetBasePlayerController))
  (bind _conversion (CallFunction|GetStringfromFolderType FolderName _outcontroller))
  (LocalVariables|SetDirName _conversion)
  (if (Class|ShlocUtils|IsPackagedGame _outcontroller)
    (return (Utilities|String|Append (Class|EFMBPLibrary|GetGameDirectoryRoot) (LocalVariables|GetDirName)))
    (else
      (return (Utilities|String|Append (Class|EFMBPLibrary|GetGameUprojectRoot) (LocalVariables|GetDirName))))))

(fn GetStringfromFolderType
  (params (FolderType :type DataFolderEnum%20Enum :default "NewEnumerator0"))
  (switch Utilities|FlowControl|Switch|SwitchonDataFolderEnum FolderType
    (:NewEnumerator0
      (return "/Data/"))
    (:NewEnumerator1
      (return "/Fonts/"))))

(fn GetFullFilePathList
  (for (_array_element _array_index) (Class|EFMBPLibrary|GetDirectoryContent (CallFunction|GetDataPath "NewEnumerator0") true false)
    (Utilities|Array|SetArrayElem (LocalVariables|GetReturnList) _array_index (Utilities|String|Append (CallFunction|GetDataPath "NewEnumerator0") _array_element) true))
  (return (LocalVariables|GetReturnList)))

(fn GetBasePlayerController
  (bind _asbp_player_controller (Utilities|Casting|CastToBP_PlayerController (Game|GetPlayerController (LocalVariables|Get__WorldContext))))
  (return _asbp_player_controller))

(fn PostLoadCSVFinished
  (params (Successful :type Boolean) (Payload :type String) (RuntimeDataTableActor :type Runtime%20Data%20Table%20Actor%20Object%20Reference)))

(fn BPUtilsAutoGenFunc
  (params (Successful :type Boolean) (Payload :type String) (RuntimeDataTableActor :type Runtime%20Data%20Table%20Actor%20Object%20Reference)))